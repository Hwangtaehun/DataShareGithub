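; BP_PlatformButton is an interactable lever that activates a linked Platform when the player presses E nearby.
; A Sphere overlap with BP_ThirdPersonCharacter enables input on the actor, and leaving the sphere disables it.
; Pressing E sets IsOn, rotates the LeverHandle to its on position and calls OnActive on the Platform, with no logic to switch it back off.
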(event `self.Sphere.OnComponentBeginOverlap`
  (params (OverlappedComponent :type "PrimitiveComponent Object Reference") (OtherActor :type "Actor Object Reference") (OtherComp :type "PrimitiveComponent Object Reference") (OtherBodyIndex :type Integer) (bFromSweep :type Boolean) (SweepResult :type "HitResult Structure (by ref)"))
  (cast `/Game/ThirdPerson/Blueprints/BP_ThirdPersonCharacter` OtherActor)
  (`self.EnableInput` (`GameplayStatics.GetPlayerController` 0)))

(event `self.Sphere.OnComponentEndOverlap`
  (params (OverlappedComponent :type "PrimitiveComponent Object Reference") (OtherActor :type "Actor Object Reference") (OtherComp :type "PrimitiveComponent Object Reference") (OtherBodyIndex :type Integer))
  (cast `/Game/ThirdPerson/Blueprints/BP_ThirdPersonCharacter` OtherActor)
  (`self.DisableInput` (`GameplayStatics.GetPlayerController` 0)))

(event `Key|E`
  (params (Key :type "Key Structure"))
  ;[1 1 1] 키보드 E를 누르면 레버가 On
  (:`Pressed`
    (set `self.IsOn` true)
    (`SceneComponent.K2_SetRelativeRotation` (`self.lever_handle`) (struct :`Pitch` -70.0) false false)
    (`/Game/MyBlueprints/BP_MovingPlatform.OnActive` (`self.Platform`))))

(fn `UserConstructionScript`)